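; BP_Player is a player Blueprint with logic for collecting tiles from a Paper2D tile map it overlaps.
; The overlap handler converts the player's position into map-local tile coordinates, flipping, offsetting and clamping Y, then passes them with CollectMap to CollectComponent.Collect.
; It also prints the tile index and coordinates for debugging.
; The node binding the handler to Hitbox overlap is never executed, so this graph does not hook it up.
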(event Custom|OnComponentBeginOverlap_Event
  (params (OverlappedComponent :type Primitive%20Component%20Object%20Reference) (OtherActor :type Actor%20Object%20Reference) (OtherComp :type Primitive%20Component%20Object%20Reference) (OtherBodyIndex :type Integer) (bFromSweep :type Boolean) (SweepResult :type Hit%20Result%20Structure%20%28by%20ref%29))
  (bind _asnew_paper_tile_map_blueprint (Utilities|Casting|CastToNewPaperTileMap_Blueprint OtherActor))
  (Development|PrintString (Utilities|String|ToString(Integer) (.TileIndex (Class|TileMapBlueprintLibrary|BreakTile (Class|PaperTileMapComponent|GetTile (Variables|/Game/BP/NewPaperTileMap_Blueprint.NewPaperTileMap_Blueprint_C|GetcollectMap _asnew_paper_tile_map_blueprint) (Math|Float|Round (/ (.X (Math|Vector|BreakVector (Math|Transform|InverseTransformLocation (Transformation|GetActorTransform _asnew_paper_tile_map_blueprint) (Transformation|GetActorLocation)))) (Variables|/Script/Paper2D.PaperTileMap|GetTileWidth (Variables|/Script/Paper2D.PaperTileMapComponent|GetTileMap (Variables|/Game/BP/NewPaperTileMap_Blueprint.NewPaperTileMap_Blueprint_C|GetcollectMap _asnew_paper_tile_map_blueprint))))) (Math|Integer|Clamp(Integer) (- (Variables|/Script/Paper2D.PaperTileMap|GetMapHeight (Variables|/Script/Paper2D.PaperTileMapComponent|GetTileMap (Variables|/Game/BP/NewPaperTileMap_Blueprint.NewPaperTileMap_Blueprint_C|GetcollectMap _asnew_paper_tile_map_blueprint))) (+ (Math|Float|Round (/ (.Y (Math|Vector|BreakVector (Math|Transform|InverseTransformLocation (Transformation|GetActorTransform _asnew_paper_tile_map_blueprint) (Transformation|GetActorLocation)))) (Variables|/Script/Paper2D.PaperTileMap|GetTileHeight (Variables|/Script/Paper2D.PaperTileMapComponent|GetTileMap (Variables|/Game/BP/NewPaperTileMap_Blueprint.NewPaperTileMap_Blueprint_C|GetcollectMap _asnew_paper_tile_map_blueprint))))) 2)) 0 (Variables|/Script/Paper2D.PaperTileMap|GetMapHeight (Variables|/Script/Paper2D.PaperTileMapComponent|GetTileMap (Variables|/Game/BP/NewPaperTileMap_Blueprint.NewPaperTileMap_Blueprint_C|GetcollectMap _asnew_paper_tile_map_blueprint)))))))))
  (Class|CollectComponent|Collect (Variables|Default|GetcollectComponent) (Variables|/Game/BP/NewPaperTileMap_Blueprint.NewPaperTileMap_Blueprint_C|GetcollectMap _asnew_paper_tile_map_blueprint) (Math|Vector2D|MakeVector2D (Math|Conversions|ToFloat(Integer) (Math|Float|Round (/ (.X (Math|Vector|BreakVector (Math|Transform|InverseTransformLocation (Transformation|GetActorTransform _asnew_paper_tile_map_blueprint) (Transformation|GetActorLocation)))) (Variables|/Script/Paper2D.PaperTileMap|GetTileWidth (Variables|/Script/Paper2D.PaperTileMapComponent|GetTileMap (Variables|/Game/BP/NewPaperTileMap_Blueprint.NewPaperTileMap_Blueprint_C|GetcollectMap _asnew_paper_tile_map_blueprint)))))) (Math|Conversions|ToFloat(Integer) (Math|Integer|Clamp(Integer) (- (Variables|/Script/Paper2D.PaperTileMap|GetMapHeight (Variables|/Script/Paper2D.PaperTileMapComponent|GetTileMap (Variables|/Game/BP/NewPaperTileMap_Blueprint.NewPaperTileMap_Blueprint_C|GetcollectMap _asnew_paper_tile_map_blueprint))) (+ (Math|Float|Round (/ (.Y (Math|Vector|BreakVector (Math|Transform|InverseTransformLocation (Transformation|GetActorTransform _asnew_paper_tile_map_blueprint) (Transformation|GetActorLocation)))) (Variables|/Script/Paper2D.PaperTileMap|GetTileHeight (Variables|/Script/Paper2D.PaperTileMapComponent|GetTileMap (Variables|/Game/BP/NewPaperTileMap_Blueprint.NewPaperTileMap_Blueprint_C|GetcollectMap _asnew_paper_tile_map_blueprint))))) 2)) 0 (Variables|/Script/Paper2D.PaperTileMap|GetMapHeight (Variables|/Script/Paper2D.PaperTileMapComponent|GetTileMap (Variables|/Game/BP/NewPaperTileMap_Blueprint.NewPaperTileMap_Blueprint_C|GetcollectMap _asnew_paper_tile_map_blueprint)))))))
  (Utilities|PrintValueVector (Math|Float|Round (/ (.X (Math|Vector|BreakVector (Math|Transform|InverseTransformLocation (Transformation|GetActorTransform _asnew_paper_tile_map_blueprint) (Transformation|GetActorLocation)))) (Variables|/Script/Paper2D.PaperTileMap|GetTileWidth (Variables|/Script/Paper2D.PaperTileMapComponent|GetTileMap (Variables|/Game/BP/NewPaperTileMap_Blueprint.NewPaperTileMap_Blueprint_C|GetcollectMap _asnew_paper_tile_map_blueprint))))) (Math|Integer|Clamp(Integer) (- (Variables|/Script/Paper2D.PaperTileMap|GetMapHeight (Variables|/Script/Paper2D.PaperTileMapComponent|GetTileMap (Variables|/Game/BP/NewPaperTileMap_Blueprint.NewPaperTileMap_Blueprint_C|GetcollectMap _asnew_paper_tile_map_blueprint))) (+ (Math|Float|Round (/ (.Y (Math|Vector|BreakVector (Math|Transform|InverseTransformLocation (Transformation|GetActorTransform _asnew_paper_tile_map_blueprint) (Transformation|GetActorLocation)))) (Variables|/Script/Paper2D.PaperTileMap|GetTileHeight (Variables|/Script/Paper2D.PaperTileMapComponent|GetTileMap (Variables|/Game/BP/NewPaperTileMap_Blueprint.NewPaperTileMap_Blueprint_C|GetcollectMap _asnew_paper_tile_map_blueprint))))) 2)) 0 (Variables|/Script/Paper2D.PaperTileMap|GetMapHeight (Variables|/Script/Paper2D.PaperTileMapComponent|GetTileMap (Variables|/Game/BP/NewPaperTileMap_Blueprint.NewPaperTileMap_Blueprint_C|GetcollectMap _asnew_paper_tile_map_blueprint))))))

(event EventBeginPlay)

(event Collision|EventActorBeginOverlap
  (params (OtherActor :type Actor%20Object%20Reference)))

(event EventTick
  (params (DeltaSeconds :type Float%20%28single-precision%29)))

(fn ConstructionScript)